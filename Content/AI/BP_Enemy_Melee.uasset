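; Melee enemy AI character that spots pawns through pawn sensing and strikes the player with a montage-based attack.
; On BeginPlay it stores its spawn location in the blackboard.
; Seeing a pawn sets it as target and starts a looping CheckTarget timer, neither function being defined here.
; Attack plays a charged-attack montage, while a separate HitDetect applies fixed damage to main characters overlapping AttackRange through their health component.
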(event `self.ReceiveBeginPlay`
  (`parent.ReceiveBeginPlay`)
  (bind _output_get (set `self.SpawnPoint` (`self.K2_GetActorLocation`)))
  (`BlackboardComponent.SetValueAsVector` (`AIBlueprintHelperLibrary.GetBlackboard` null) (`self.SpawnPointKey`) _output_get))

(event `self.PawnSensing.OnSeePawn`
  (params (Pawn :type "Pawn Object Reference"))
  (`self.SetTarget` Pawn)
  (`KismetSystemLibrary.K2_SetTimer` null "CheckTarget" 0.5 true))

(fn `Attack`
  (`self.PlayAnimMontage` "/Game/Variant_Combat/Anims/AM_ChargedAttack.AM_ChargedAttack"))

(fn `HitDetect`
  (for _array_element (`PrimitiveComponent.GetOverlappingActors` (`self.AttackRange`) "/Game/BPS/BPS_character/BP_MainCharacter.BP_MainCharacter_C")
    (`/Game/BPS/BP_componentHealt.DamageAmount` (`self.GetComponentByClass` _array_element "/Game/BPS/BP_componentHealt.BP_componentHealt_C") 20.0)))

(fn `UserConstructionScript`
  (`parent.UserConstructionScript`))