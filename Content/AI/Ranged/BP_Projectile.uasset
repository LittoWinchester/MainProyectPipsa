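; BP_Projectile is a projectile, filed under ranged AI, that damages actors it touches.
; Each Tick it offsets itself by Direction times Speed, without sweep or delta-time scaling, and its life span is five seconds.
; When its Sphere overlaps an actor with a BP_componentHealt, it prints a debug message and applies fixed damage through that component, without destroying itself.
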(event `self.ReceiveBeginPlay`
  (`self.SetLifeSpan` 5.0))

(event `self.ReceiveActorBeginOverlap`
  (params (OtherActor :type "Actor Object Reference")))

(event `self.ReceiveTick`
  (params (DeltaSeconds :type "Float (single-precision)"))
  (`self.K2_AddActorLocalOffset` (* (`self.Direction`) (`self.Speed`))))

(event `self.Sphere.OnComponentBeginOverlap`
  (params (OverlappedComponent :type "PrimitiveComponent Object Reference") (OtherActor :type "Actor Object Reference") (OtherComp :type "PrimitiveComponent Object Reference") (OtherBodyIndex :type Integer) (bFromSweep :type Boolean) (SweepResult :type "HitResult Structure (by ref)"))
  (bind _returnvalue (`self.GetComponentByClass` OtherActor "/Game/BPS/BP_componentHealt.BP_componentHealt_C"))
  (`/Engine/EditorBlueprintResources/StandardMacros.IsValid` _returnvalue
    (:`Is Valid`
      (`KismetSystemLibrary.PrintString` "Le pegué a alguien." true true (struct :`R` 0.283476 :`G` 1.0 :`A` 1.0))
      (`/Game/BPS/BP_componentHealt.DamageAmount` _returnvalue 105.0))))

(fn `UserConstructionScript`)