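; Ranged enemy that fires projectiles at the main character.
; Attack plays a pistol-fire montage, computes a normalized direction to the BP_MainCharacter actor, then spawns a BP_Projectile at ProjectileSpawnPos with that direction.
; A separate Rotate function turns the enemy 90 degrees in yaw per call.
; The event graph is empty, so neither Attack nor Rotate is called within this Blueprint.
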(event `self.ReceiveBeginPlay`)

(fn `Attack`
  (`self.PlayAnimMontage` "/Game/Characters/Mannequins/Anims/Pistol/MM_Pistol_Fire_Montage.MM_Pistol_Fire_Montage")
  (`self.Set Attack Direction`)
  (`|SpawnActorFromClass` "/Game/AI/Ranged/BP_Projectile.BP_Projectile_C" (`KismetMathLibrary.MakeTransform` (`SceneComponent.K2_GetComponentLocation` (`self.ProjectileSpawnPos`))) "Undefined" "MultiplyWithRoot" null (`self.AttackDirection`) null))

(fn `Rotate`
  (bind (_returnvalue_roll _returnvalue_pitch _returnvalue_yaw) (`KismetMathLibrary.BreakRotator` (`self.K2_GetActorRotation`)))
  (`self.K2_SetActorRotation` (`KismetMathLibrary.MakeRotator` _returnvalue_roll _returnvalue_pitch (+ _returnvalue_yaw 90.0))))

(fn `Set Attack Direction`
  (bind _returnvalue (`GameplayStatics.GetActorOfClass` "/Game/BPS/BPS_character/BP_MainCharacter.BP_MainCharacter_C"))
  (set `self.AttackDirection` (`KismetMathLibrary.Normal` (- (`self.K2_GetActorLocation` _returnvalue) (`self.K2_GetActorLocation`)))))

(fn `UserConstructionScript`
  (`parent.UserConstructionScript`))