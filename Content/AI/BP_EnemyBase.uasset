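; BP_EnemyBase is an enemy base Blueprint that rewards the player with XP when it dies.
; On BeginPlay it binds GrantXP to the health component's death event.
; GrantXP finds BP_MainCharacter with GetActorOfClass, passes XPReward and the player's level to RefreshXP, then destroys the enemy.
; Attack and the PawnSensing see-pawn event are empty, with no behavior in this class.
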(event `self.ReceiveBeginPlay`
  (add `/Game/BPS/BP_componentHealt.OnDeath` (`self.BP_componentHealt`) (delegate `GrantXP`)))

(event `GrantXP`
  (`|ExecutionSequence`
    (:`then_0`
      (bind _returnvalue (`GameplayStatics.GetActorOfClass` "/Game/BPS/BPS_character/BP_MainCharacter.BP_MainCharacter_C"))
      (`/Game/BPS/BPS_character/BP_MainCharacter.RefreshXP` _returnvalue (`/Game/BPS/BPS_character/BP_MainCharacter.Level Player` _returnvalue) (`self.XPReward`)))
    (:`then_1`
      (`self.K2_DestroyActor`))))

(event `self.PawnSensing.OnSeePawn`
  (params (Pawn :type "Pawn Object Reference")))

(fn `Attack`)

(fn `UserConstructionScript`)