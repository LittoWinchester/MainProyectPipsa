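; Health component that tracks current HP for whatever owns it, starting at HPMax on BeginPlay.
; HealAmount adds HP up to a hard-coded cap of 100, independent of HPMax.
; DamageAmount subtracts HP and returns the result with a dead flag.
; At zero or below it calls OnDeath and reports zero, though stored HP is not clamped.
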(event `self.ReceiveBeginPlay`
  (set `self.HP_Actual` (`self.HP_Max`)))

(fn `DamageAmount`
  (params (AmountDMG :type "Float (double-precision)"))
  (returns (`Actual HP` :type "Float (double-precision)") (`Dead?` :type Boolean))
  (bind _output_get (set `self.HP_Actual` (- (`self.HP_Actual`) AmountDMG)))
  (if (<= _output_get 0.0)
    (`self.OnDeath`)
    (return 0.0 true)
    (else
      (return _output_get false))))

(fn `HealAmount`
  (params (`Amount Heal` :type "Float (double-precision)"))
  (returns (`HP actual` :type "Float (double-precision)"))
  (if (not (>= (`self.HP_Actual`) 100.0))
    (bind _output_get (set `self.HP_Actual` (+ (`self.HP_Actual`) `Amount Heal`)))
    (if (>= _output_get 100.0)
      (bind _output_get_2 (set `self.HP_Actual` 100.0))
      (return _output_get_2)
      (else
        (return _output_get)))))