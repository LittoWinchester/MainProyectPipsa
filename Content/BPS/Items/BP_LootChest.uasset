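; BP_LootChest is a loot chest actor that gives its items to the main character when touched, then destroys itself.
; It becomes interactable one second after BeginPlay.
; A box overlap by an actor implementing BPI_Forja adds each DroppedItems entry to the inventory of the BP_MainCharacter found with GetActorOfClass, not to the overlapping actor.
; The Loot event is empty.
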(event `self.ReceiveBeginPlay`
  (`KismetSystemLibrary.Delay` 1.0)
  (set `self.bInteractable?` true))

(event `self.Box.OnComponentBeginOverlap`
  (params (OverlappedComponent :type "PrimitiveComponent Object Reference") (OtherActor :type "Actor Object Reference") (OtherComp :type "PrimitiveComponent Object Reference") (OtherBodyIndex :type Integer) (bFromSweep :type Boolean) (SweepResult :type "HitResult Structure (by ref)"))
  (if (and (`KismetSystemLibrary.DoesImplementInterface` OtherActor "/Game/BPS/Forja/BPI_Forja.BPI_Forja_C") (`self.bInteractable?`))
    (for _array_element (`self.DroppedItems`)
      (bind _returnvalue (`GameplayStatics.GetActorOfClass` "/Game/BPS/BPS_character/BP_MainCharacter.BP_MainCharacter_C"))
      (`/Game/BPS/BPS_character/BP_MainCharacter.AddToInventory` _returnvalue _array_element))
    (`self.K2_DestroyActor`)))

(event `self.Box.OnComponentEndOverlap`
  (params (OverlappedComponent :type "PrimitiveComponent Object Reference") (OtherActor :type "Actor Object Reference") (OtherComp :type "PrimitiveComponent Object Reference") (OtherBodyIndex :type Integer)))

(event `/Game/BPS/Data/Drops/BPI_Loot.Loot`)

(fn `UserConstructionScript`)