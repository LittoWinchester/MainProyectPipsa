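; Base NPC Blueprint that offers chat and an optional quest to actors entering its collision.
; On BeginPlay it caches BP_MainCharacter and, if flagged as having a quest, copies the QuestN row from DT_Quest into its variables.
; Overlap begin messages the other actor with chat and any quest name; overlap end sends an empty message and closes the quest interface.
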(event `self.ReceiveBeginPlay`
  (bind _returnvalue (`GameplayStatics.GetActorOfClass` "/Game/BPS/BPS_character/BP_MainCharacter.BP_MainCharacter_C"))
  (set `self.Char` _returnvalue)
  (`self.NPC_LoadQuest`))

(event `self.Collision.OnComponentBeginOverlap`
  (params (OverlappedComponent :type "PrimitiveComponent Object Reference") (OtherActor :type "Actor Object Reference") (OtherComp :type "PrimitiveComponent Object Reference") (OtherBodyIndex :type Integer) (bFromSweep :type Boolean) (SweepResult :type "HitResult Structure (by ref)"))
  (bind _output_get (set `self.Overlap Npc` true))
  (if (`self.NPC had Quest?`)
    (message `/Game/BPS/NPCs/BPI_NPC.FN_NPC_BASE_questname` OtherActor _output_get (`self.Quest_n`) (`self.chatNPC`) true)
    (else
      (message `/Game/BPS/NPCs/BPI_NPC.FN_NPC_BASE_questname` OtherActor _output_get "None" (`self.chatNPC`) false))))

(event `self.Collision.OnComponentEndOverlap`
  (params (OverlappedComponent :type "PrimitiveComponent Object Reference") (OtherActor :type "Actor Object Reference") (OtherComp :type "PrimitiveComponent Object Reference") (OtherBodyIndex :type Integer))
  (message `/Game/BPS/NPCs/BPI_NPC.FN_NPC_BASE_questname` OtherActor false "None" "" false)
  (set `self.Overlap Npc` false)
  (message `/Game/BPS/NPCs/BPI_NPC.FN_OpenQuestInterface` OtherActor false))

(fn `NPC_LoadQuest`
  (if (`self.NPC had Quest?`)
    (bind _returnvalue (`|GetDataTableRow` "/Game/BPS/Data/Quest/DT_Quest.DT_Quest" (`self.Quest_n`))
      (:`then`
        (set `self.HaceQuest?` true)
        (set `self.Out Row Name Quest` (break `/Game/BPS/Data/Quest/STR_QuestData` _returnvalue))
        (set `self.Out Row Description` (`.Description_18_610D0ABC4AEA5B4AAE41C7B1BAC46500` (break `/Game/BPS/Data/Quest/STR_QuestData` _returnvalue)))
        (set `self.Out Row Requirement` (`.Requirement_24_D989018E4BB84C5BDD6FA5A6729CD9E3` (break `/Game/BPS/Data/Quest/STR_QuestData` _returnvalue)))
        (set `self.Out Row Amount` (`.Amount_20_17DD9C0445519560CF97E8971BF36057` (break `/Game/BPS/Data/Quest/STR_QuestData` _returnvalue)))
        (set `self.Out Row Reward` (`.Reward_25_007A04C4454D9F0F26BE09A90C3ABBFE` (break `/Game/BPS/Data/Quest/STR_QuestData` _returnvalue)))
        (set `self.Out Row Experience` (`.Experience_22_8C83F5CF41526279C7598D814E8545BF` (break `/Game/BPS/Data/Quest/STR_QuestData` _returnvalue)))
        (set `self.Out Row IMG` (`.IMG_23_DF3D5B9B4D4E85C3A8C0ACA8228D8C16` (break `/Game/BPS/Data/Quest/STR_QuestData` _returnvalue)))
        (set `self.Out Row Completed` (`.Completed_16_3339F5684339F8FE7C4AF7ACDB8842EE` (break `/Game/BPS/Data/Quest/STR_QuestData` _returnvalue))))
      (:`RowNotFound`
        (set `self.HaceQuest?` false)))))

(fn `UserConstructionScript`)